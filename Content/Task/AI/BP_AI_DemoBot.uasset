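; BP_AI_DemoBot is a demo AI bot that emits noise for perception testing.
; Every tick it calls MakeNoise at its own location with a limited range, using itself as instigator.
; Its AIPerception update and forgotten events are stubs, with debug prints and a sound cue left disconnected, so it does not react to what it perceives.
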(event `self.ReceiveTick`
  (params (DeltaSeconds :type "Float (single-precision)"))
  (`self.MakeNoise` 1.0 self (`self.K2_GetActorLocation` self) 500.0))

(event `self.AIPerception.OnPerceptionUpdated`
  (params (UpdatedActors :type "Array of Actor Object Reference (by ref)"))
  (for _array_element UpdatedActors
    _))

(event `self.AIPerception.OnTargetPerceptionForgotten`
  (params (Actor :type "Actor Object Reference")))

(event `self.AIPerception.OnTargetPerceptionUpdated`
  (params (Actor :type "Actor Object Reference") (Stimulus :type "AIStimulus Structure")))

(fn `UserConstructionScript`)